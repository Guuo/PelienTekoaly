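; BP_Boid is a robot AI character that flocks while following the player, using steering behaviour components.
; On Tick, when CurrentAction matches the flocking state, it turns toward the player and SbBoidComponent calculates its new position from its CharacterMovement.
; An unconnected graph section holds distance-based logic that switches between path patrol, a delayed face-the-player pause and seeking, but it never runs.
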(event `self.ReceiveTick`
  (params (DeltaSeconds :type "Float (single-precision)"))
  (if (`|EnumEquality` (`self.CurrentAction`) "NewEnumerator6")
    ;[1 1 1] Make robot character follow player when flocking.
    (bind _output_get (set `self.VelocityForFlocking` (- (`CharacterMovementComponent.GetLastUpdateLocation` (`Character.CharacterMovement` (`GameplayStatics.GetPlayerCharacter` 0))) (`CharacterMovementComponent.GetLastUpdateLocation` (`self.CharacterMovement`)))))
    (`self.K2_SetActorRotation` (`KismetMathLibrary.Conv_VectorToRotator` _output_get))
    ;[1 1 1] Flock.
    (`/Game/Blueprints/AI_Blueprints/SteeringBehaviourComponents/sbBoidComponent.calculateNewPosition` (`self.sbBoidComponent`) (`self.CharacterMovement`) null)))

(fn `UserConstructionScript`)