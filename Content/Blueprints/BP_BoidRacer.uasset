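; BP_BoidRacer is the possessable pawn for a racing minigame, with movement driven by its SbRacing object.
; On BeginPlay it binds to the CustomPlayerController's begin-racing event, which has player controller 0 possess it.
; Possession and unpossession switch Tick on and off; each tick passes CharacterMovement to SbRacing to calculate the new position.
; Space bar adds a forward impulse through CharacterMovement.
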(event `self.ReceiveTick`
  (params (DeltaSeconds :type "Float (single-precision)"))
  (`/Game/Blueprints/AI_Blueprints/SteeringBehaviourComponents/sbRacing.Calculate New Position` (`self.sbRacing`) (`self.CharacterMovement`) DeltaSeconds))

(event `Key|SpaceBar`
  (params (Key :type "Key Structure"))
  (:`Pressed`
    (`CharacterMovementComponent.AddImpulse` (`self.CharacterMovement`) (* (`self.GetActorForwardVector`) 5000.0) false)))

(event `self.ReceiveBeginPlay`
  (bind _ascustom_player_controller (cast `/Game/Blueprints/CustomPlayerController` (`GameplayStatics.GetPlayerController` 0)))
  (add `/Game/Blueprints/CustomPlayerController.BeginRacingMiniGame` _ascustom_player_controller (delegate `BeginRacingMiniGame_Event`)))

(event `self.ReceivePossessed`
  (params (NewController :type "Controller Object Reference"))
  (`self.SetActorTickEnabled` true))

(event `BeginRacingMiniGame_Event`
  (`Controller.Possess` (`GameplayStatics.GetPlayerController` 0) self))

(event `self.ReceiveUnpossessed`
  (params (OldController :type "Controller Object Reference"))
  (`self.SetActorTickEnabled` false))

(fn `UserConstructionScript`)