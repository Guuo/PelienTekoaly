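; Dialog component for an AI_Character that runs branching conversations with the player.
; While the owner is in its dialog action, Tick checks distance and facing, then opens WBP_DialogGUI or closes it out of range.
; A semicolon-delimited text file becomes a flat array, walked in five-field strides to show AI phrases and up to three replies.
; Reply tags adjust Attitude or store key-value memories, which a debug event prints.
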(event `self.ReceiveBeginPlay`
  ;[1 1 1] Korvaa interfacella tms. jos oikea käyttötarkotus
  (bind _asai_character (cast `/Game/ThirdPersonBP/Blueprints/AI_Character` (`self.GetOwner`)))
  (set `self.Owner` _asai_character)
  (add `/Game/ThirdPersonBP/Blueprints/ThirdPersonCharacter.OnRequestDebugInfo` (`self.PlayerActor`) (`|CreateDelegate` :!event `DialogDebugPrintOut`)))

(event `self.ReceiveTick`
  (params (DeltaSeconds :type "Float (single-precision)"))
  (if (`|EnumEquality` (`/Game/ThirdPersonBP/Blueprints/AI_Character.CurrentAction` (`self.Owner`)) "NewEnumerator8")
    ;[1 1 1] Only discuss with player if he/she is close enough.
    (bind _outcome (`self.IsWithinDiscussionRange`))
    (if _outcome
      ;[1 1 1] Check whether discussion has started already or not.
      (if (== (`self.CurrentAIPhraseID`) 0)
        ;[1 1 1] If not, set up the dialog tree and  show discussion GUI ...
        (`self.SetupDialogTree` (`self.DialogFile`))
        (if (`KismetSystemLibrary.IsValid` (`self.DialogTreeGUI`))
          ;[1 1 1] Bind event to handle AI's responses based on event dispatched by GUI when player speaks.
          (add `/Game/UI/WBP_DialogGUI.PlayerSpoke_ED` (`self.DialogTreeGUI`) (delegate `Playerspoke`))))
      (else
        (`self.DisableDialogTree`)))))

(event `DialogDebugPrintOut`
  (bind _dialogmemorytags (`self.DialogMemoryTags`))
  (bind (_value _returnvalue) (`BlueprintMapLibrary.Map_Find` _dialogmemorytags "POMMISUOJAPANOT"))
  (bind (_value_2 _returnvalue_2) (`BlueprintMapLibrary.Map_Find` _dialogmemorytags "LAINASI_RAHAA"))
  (bind (_value_3 _returnvalue_3) (`BlueprintMapLibrary.Map_Find` _dialogmemorytags "HASLAYS"))
  (bind (_value_4 _returnvalue_4) (`BlueprintMapLibrary.Map_Find` _dialogmemorytags "LAINATTU_SUMMA"))
  ;[1 1 1] Debug output
  (if _returnvalue_3
    (`KismetSystemLibrary.PrintString` (`KismetStringLibrary.Concat_StrStr` "Pulkkisen mielestä Sauli " _value_3) true true (struct :`G` 0.66 :`B` 1.0 :`A` 1.0) 10.0))
  (if _returnvalue
    (`KismetSystemLibrary.PrintString` (`KismetStringLibrary.Concat_StrStr` "Pulkkisen mielestä Sauli " _value) true true (struct :`G` 0.66 :`B` 1.0 :`A` 1.0) 10.0))
  (if _returnvalue_2
    (`KismetSystemLibrary.PrintString` (`KismetStringLibrary.Concat_StrStr` "Rahanlainauksen status: " _value_2) true true (struct :`G` 0.66 :`B` 1.0 :`A` 1.0) 10.0))
  (if _returnvalue_4
    (`KismetSystemLibrary.PrintString` (`KismetStringLibrary.Concat_StrStr` "Lainatun rahan määrä: " _value_4) true true (struct :`G` 0.66 :`B` 1.0 :`A` 1.0) 10.0)
    (else
      (`KismetSystemLibrary.PrintString` "Lainatun rahan määrä: 0EUR" true true (struct :`G` 0.66 :`B` 1.0 :`A` 1.0) 10.0)))
  (`KismetSystemLibrary.PrintString` (`KismetStringLibrary.Concat_StrStr` "Pulkkisen suhtautuminen Sauliin: " (`KismetStringLibrary.Conv_DoubleToString` (`self.Attitude`))) true true (struct :`G` 0.66 :`B` 1.0 :`A` 1.0) 10.0))

(event `Playerspoke`
  (params (PlayerChoice :type Integer))
  ;[1 1 1] After every response of the player ...
  (bind (_nextnode _responsetag _responseinfo) (`self.UpdateTree` PlayerChoice))
  (`self.ProcessResponseMetadata` _responsetag _responseinfo)
  ;[1 1 1] .. either continue or terminate the discussion based on the response.
  (if (not (> _nextnode 0))
    (`self.DisableDialogTree`)
    (switch `string` (`self.DialogFile`)
      (:`dialogtesti1.txt`
        (set `/Game/ThirdPersonBP/Blueprints/AI_Character.CurrentAction` "NewEnumerator0" (`self.Owner`))))))

(fn `DisableDialogTree`
  (bind _returnvalue (`GameplayStatics.GetPlayerController` 0))
  (bind _dialogtreegui (`self.DialogTreeGUI`))
  ;[1 1 1] Remove dialog tree and return interaction to its original mode.
  (if (`KismetSystemLibrary.IsValid` _dialogtreegui)
    (`Widget.RemoveFromParent` _dialogtreegui)
    (`WidgetBlueprintLibrary.SetInputMode_GameOnly` _returnvalue)
    (set `PlayerController.bShowMouseCursor` false _returnvalue)
    (set `self.CurrentAIPhraseID` 0)))

(fn `IsWithinDiscussionRange`
  (returns (Outcome :type Boolean))
  (locals (DiscussionRange :type "Float (double-precision)" :default 600.0) (MinDiscussionRange :type "Float (double-precision)" :default -0.5) (MaxDiscussionRange :type "Float (double-precision)" :default -0.25) (MaxDiscussionAngle :type "Float (double-precision)" :default 90.0))
  (bind _returnvalue (`KismetMathLibrary.Conv_RotatorToVector` (`Actor.K2_GetActorRotation` (`GameplayStatics.GetPlayerCharacter` 0))))
  (bind _returnvalue_2 (`KismetMathLibrary.Conv_RotatorToVector` (`Actor.K2_GetActorRotation` (`self.Owner`))))
  (return (and (`KismetMathLibrary.InRange_FloatFloat` (/ (`KismetMathLibrary.Dot_VectorVector` _returnvalue_2 _returnvalue) (+ (`KismetMathLibrary.VSize` _returnvalue_2) (`KismetMathLibrary.VSize` _returnvalue))) (`local.MinDiscussionRange`) (`local.MaxDiscussionRange`)) (< (`KismetMathLibrary.Vector_Distance` (`Actor.K2_GetActorLocation` (`self.Owner`)) (`Actor.K2_GetActorLocation` (`GameplayStatics.GetPlayerCharacter` 0))) (`local.DiscussionRange`)) (< (`KismetMathLibrary.Dot_VectorVector` (`Actor.GetActorForwardVector` (`self.Owner`)) (`KismetMathLibrary.Normal` (- (`Actor.K2_GetActorLocation` (`self.Owner`)) (`Actor.K2_GetActorLocation` (`GameplayStatics.GetPlayerCharacter` 0))))) (`KismetMathLibrary.DegCos` (`local.MaxDiscussionAngle`))))))

(fn `ProcessResponseMetadata`
  (params (Tag :type String) (Info :type String))
  (locals (TagArray :type "Array of String") (InfoArray :type "Array of String") (CurrentIndex :type Integer))
  (bind _currentindex (`local.CurrentIndex`))
  (set `local.TagArray` (`KismetStringLibrary.ParseIntoArray` Tag ":"))
  (set `local.InfoArray` (`KismetStringLibrary.ParseIntoArray` Info ":"))
  (for (_array_element _array_index) (`local.TagArray`)
    (set `local.CurrentIndex` _array_index)
    (switch `string` _array_element
      (:`Default`
        ;[1 1 1] All other tags are treated as kv-pairs
        (`BlueprintMapLibrary.Map_Add` (`self.DialogMemoryTags`) (`|GetArrayItem` (`local.TagArray`) _currentindex) (`|GetArrayItem` (`local.InfoArray`) _currentindex)))
      (:`CHANGE_ATTITUDE`
        (switch `string` (`|GetArrayItem` (`local.InfoArray`) (`local.CurrentIndex`))
          (:`POSITIVE`
            (set `self.Attitude` (+ (`self.Attitude`) 0.1)))
          (:`NEGATIVE`
            (set `self.Attitude` (- (`self.Attitude`) 0.1))))))))

(fn `SetupDialogTree`
  (params (DialogFile :type String))
  (bind _returnvalue (`GameplayStatics.GetPlayerController` 0))
  (bind _dialogtreegui (`self.DialogTreeGUI`))
  (bind _pc1_t (`/Game/UI/WBP_DialogGUI.PC1_T` _dialogtreegui))
  (bind _pc2_t (`/Game/UI/WBP_DialogGUI.PC2_T` _dialogtreegui))
  (bind _pc3_t (`/Game/UI/WBP_DialogGUI.PC3_T` _dialogtreegui))
  ;[1 1 1] Check that the tree for the dialog is valid and set dialog tree.
  (set `self.DialogFile` DialogFile)
  (if (`KismetStringLibrary.Contains` (`self.DialogFile`) "Dialog")
    ;[1 1 1] Create dialog tree HUD and add it to viewport
    (bind _returnvalue_2 (`|CreateWidget` "/Game/UI/WBP_DialogGUI.WBP_DialogGUI_C"))
    (bind _output_get (set `self.DialogTreeGUI` _returnvalue_2))
    (`UserWidget.AddToViewport` _output_get 0)
    (`self.ShowAnswerGUIWidgets`)
    ;[1 1 1] Set up interaction.
    (`WidgetBlueprintLibrary.SetInputMode_GameAndUIEx` _returnvalue null)
    (set `PlayerController.bShowMouseCursor` true _returnvalue)
    ;[1 1 1] Load the dialog tree from the source txt-file and parse it into an array.
    (bind _savetexta (`DialogLoader.FileLoadString` (`self.DialogFile`)))
    (bind _output_get_2 (set `self.DialogArray` (`KismetStringLibrary.ParseIntoArray` _savetexta ";")))
    ;[1 1 1] Set the initial AI´s phrase.
    (bind _output_get_3 (set `self.AIPhrase` (`/Game/UI/WBP_DialogGUI.AI_Phrase_TB` _dialogtreegui)))
    (`TextBlock.SetText` _output_get_3 (`KismetTextLibrary.Conv_StringToText` (`|GetArrayItem` _output_get_2 1)))
    (bind _output (`|GetArrayItem` _output_get_2 6))
    ;[1 1 1] Set initial first answer option for player.
    (if (!= _output "-")
      (`TextBlock.SetText` _pc1_t (`KismetTextLibrary.Conv_StringToText` _output))
      (else
        (`/Game/UI/WBP_DialogGUI.HideGUIWidget` (`self.DialogTreeGUI`) (`Widget.GetParent` _pc1_t))))
    (bind _output_2 (`|GetArrayItem` _output_get_2 11))
    ;[1 1 1] Set initial second answer option for player, if there is one..
    (if (!= _output_2 "-")
      (`TextBlock.SetText` _pc2_t (`KismetTextLibrary.Conv_StringToText` _output_2))
      (else
        (`/Game/UI/WBP_DialogGUI.HideGUIWidget` (`self.DialogTreeGUI`) (`Widget.GetParent` _pc2_t))))
    (bind _output_3 (`|GetArrayItem` _output_get_2 16))
    ;[1 1 1] Set initial third answer option for player, if there is one.
    (if (!= _output_3 "-")
      (`TextBlock.SetText` _pc3_t (`KismetTextLibrary.Conv_StringToText` _output_3))
      (else
        (`/Game/UI/WBP_DialogGUI.HideGUIWidget` (`self.DialogTreeGUI`) (`Widget.GetParent` _pc3_t))))
    ;[1 1 1] Make sure discussion starts from the first phrase.
    (set `self.CurrentAIPhraseID` 1)
    (else
      (set `self.CurrentAIPhraseID` 0))))

(fn `ShowAnswerGUIWidgets`
  (bind _dialogtreegui (`self.DialogTreeGUI`))
  (`/Game/UI/WBP_DialogGUI.ShowGUIWidget` _dialogtreegui (`/Game/UI/WBP_DialogGUI.Player_Choice1_B` _dialogtreegui))
  (`/Game/UI/WBP_DialogGUI.ShowGUIWidget` (`self.DialogTreeGUI`) (`/Game/UI/WBP_DialogGUI.Player_Choice2_B` _dialogtreegui))
  (`/Game/UI/WBP_DialogGUI.ShowGUIWidget` (`self.DialogTreeGUI`) (`/Game/UI/WBP_DialogGUI.Player_Choice3_B` _dialogtreegui)))

(fn `UpdateTree`
  (params (SelectedResponse :type Integer))
  (returns (NextNode :type Integer) (ResponseTag :type String) (ResponseInfo :type String))
  (bind _dialogarray (`self.DialogArray`))
  (bind _dialogarray_2 (`self.DialogArray`))
  (bind _dialogarray_3 (`self.DialogArray`))
  (bind _dialogtreegui (`self.DialogTreeGUI`))
  (bind _pc1_t (`/Game/UI/WBP_DialogGUI.PC1_T` _dialogtreegui))
  (bind _pc2_t (`/Game/UI/WBP_DialogGUI.PC2_T` _dialogtreegui))
  (bind _pc3_t (`/Game/UI/WBP_DialogGUI.PC3_T` _dialogtreegui))
  (bind _returnvalue (- (+ (* SelectedResponse 5) (* (`self.CurrentAIPhraseID`) 5)) 1))
  (bind _returnvalue_2 (`KismetStringLibrary.Conv_StringToInt` (`|GetArrayItem` (`self.DialogArray`) _returnvalue)))
  (bind _returnvalue_3 (- (* (`KismetStringLibrary.Conv_StringToInt` (`|GetArrayItem` _dialogarray_2 _returnvalue)) 5) 4))
  (bind _output (`|GetArrayItem` _dialogarray_3 (+ _returnvalue_3 5)))
  (bind _output_2 (`|GetArrayItem` _dialogarray_3 (+ _returnvalue_3 10)))
  (bind _output_3 (`|GetArrayItem` _dialogarray_3 (+ _returnvalue_3 15)))
  (`self.ShowAnswerGUIWidgets`)
  ;[1 1 1] Extract tag and info out of a discussion piece.
  (set `self.Tag` (`|GetArrayItem` _dialogarray (- _returnvalue 2)))
  (set `self.Info` (`|GetArrayItem` _dialogarray (- _returnvalue 1)))
  ;[1 1 1] Check whether dialog continues and exit with true if so..
  (if (> _returnvalue_2 0)
    ;[1 1 1] Fetch next AI phrase and place it to the GUI.
    (`TextBlock.SetText` (`self.AIPhrase`) (`KismetTextLibrary.Conv_StringToText` (`|GetArrayItem` _dialogarray_2 _returnvalue_3)))
    ;[1 1 1] Fetch first player response option and place it to the GUI.
    (if (!= _output "-")
      (`TextBlock.SetText` _pc1_t (`KismetTextLibrary.Conv_StringToText` _output))
      (else
        (`/Game/UI/WBP_DialogGUI.HideGUIWidget` (`self.DialogTreeGUI`) (`Widget.GetParent` _pc1_t))))
    ;[1 1 1] Fetch second player response option and place it to the GUI.
    (if (!= _output_2 "-")
      (`TextBlock.SetText` _pc2_t (`KismetTextLibrary.Conv_StringToText` _output_2))
      (else
        (`/Game/UI/WBP_DialogGUI.HideGUIWidget` (`self.DialogTreeGUI`) (`Widget.GetParent` _pc2_t))))
    ;[1 1 1] Fetch third player response option and place it to the GUI.
    (if (!= _output_3 "-")
      (`TextBlock.SetText` _pc3_t (`KismetTextLibrary.Conv_StringToText` _output_3))
      (else
        (`/Game/UI/WBP_DialogGUI.HideGUIWidget` (`self.DialogTreeGUI`) (`Widget.GetParent` _pc3_t))))
    ;[1 1 1] Update current AI phrase and return with ID on question to see whether dialog is over and with what outcome.
    (set `self.CurrentAIPhraseID` (`KismetStringLibrary.Conv_StringToInt` (`|GetArrayItem` _dialogarray_2 _returnvalue)))
    (return _returnvalue (`self.Tag`) (`self.Info`))
    (else
      (return _returnvalue_2 (`self.Tag`) (`self.Info`)))))