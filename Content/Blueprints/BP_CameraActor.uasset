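; Follow camera for the racing minigame, tracking the BP_BoidRacer found at BeginPlay.
; It becomes the blended view target when CustomPlayerController fires its BeginRacingMiniGame event.
; Every tick it eases its X and Y toward the racer with a fixed-alpha lerp, keeping height and rotation.
; Disconnected leftover logic once authored the racer's path through mouse traces, numbered text markers and a save game.
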(event `self.ReceiveBeginPlay`
  (bind _returnvalue (`GameplayStatics.GetActorOfClass` "/Game/Blueprints/BP_BoidRacer.BP_BoidRacer_C"))
  (set `self.Racer` _returnvalue)
  (bind _ascustom_player_controller (cast `/Game/Blueprints/CustomPlayerController` (`GameplayStatics.GetPlayerController` 0)))
  (add `/Game/Blueprints/CustomPlayerController.BeginRacingMiniGame` _ascustom_player_controller (delegate `BeginRacingMiniGame_Event`)))

(event `BeginRacingMiniGame_Event`
  (`PlayerController.SetViewTargetWithBlend` (`GameplayStatics.GetPlayerController` 0) self 2.0 "VTBlend_Linear" 2.0 false))

(event `self.ReceiveTick`
  (params (DeltaSeconds :type "Float (single-precision)"))
  (`self.K2_SetActorTransform` (`KismetMathLibrary.MakeTransform` (`KismetMathLibrary.MakeVector` (`KismetMathLibrary.Lerp` (.x (.location (`self.GetTransform`))) (.x (.location (`self.GetTransform` (`self.Racer`)))) 0.05) (`KismetMathLibrary.Lerp` (.y (.location (`self.GetTransform`))) (.y (.location (`self.GetTransform` (`self.Racer`)))) 0.05) (.z (.location (`self.GetTransform`)))) (.rotation (`self.GetTransform`)))))

(event `Key|M`
  (params (Key :type "Key Structure"))
  ;[1 1 1] Inputs were used to get a path for the racer to follow
)

(event `Key|N`
  (params (Key :type "Key Structure"))
  ;[1 1 1] Inputs were used to get a path for the racer to follow
)

(event `Key|NumPadZero`
  (params (Key :type "Key Structure"))
  ;[1 1 1] Inputs were used to get a path for the racer to follow
)

(fn `UserConstructionScript`)